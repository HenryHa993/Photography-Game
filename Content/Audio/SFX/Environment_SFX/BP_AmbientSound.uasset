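; BP_AmbientSound is a placeable ambient sound actor that plays an assigned sound cue while the photo character is inside its box trigger.
; The construction script applies the per-instance cue, attenuation and box extent to the audio and collision components.
; If PlayOnStart is set, BeginPlay starts playback at a random offset within the cue's duration.
; Box entry plays the sound from the beginning, and exit stops it.
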(event `self.ReceiveBeginPlay`
  (bind _output_get (set `self.StartTime` (`KismetMathLibrary.RandomFloatInRange` 0.0 (`SoundBase.Duration` (`self.SoundCue`)))))
  (if (`self.PlayOnStart`)
    (`AudioComponent.Play` (`self.AmbientSound`) _output_get)))

(event `self.BoxCollision.OnComponentEndOverlap`
  (params (OverlappedComponent :type "PrimitiveComponent Object Reference") (OtherActor :type "Actor Object Reference") (OtherComp :type "PrimitiveComponent Object Reference") (OtherBodyIndex :type Integer))
  (cast `/Game/Core/Characters/Player/BP_PhotoCharacterBase` OtherActor)
  (`AudioComponent.Stop` (`self.AmbientSound`)))

(event `self.BoxCollision.OnComponentBeginOverlap`
  (params (OverlappedComponent :type "PrimitiveComponent Object Reference") (OtherActor :type "Actor Object Reference") (OtherComp :type "PrimitiveComponent Object Reference") (OtherBodyIndex :type Integer) (bFromSweep :type Boolean) (SweepResult :type "HitResult Structure (by ref)"))
  (cast `/Game/Core/Characters/Player/BP_PhotoCharacterBase` OtherActor)
  (`AudioComponent.Play` (`self.AmbientSound`) 0.0))

(fn `UserConstructionScript`
  (`AudioComponent.SetSound` (`self.AmbientSound`) (`self.SoundCue`))
  (set `AudioComponent.AttenuationSettings` (`self.AmbientSoundAttenuation`) (`self.AmbientSound`))
  (`BoxComponent.SetBoxExtent` (`self.BoxCollision`) (`self.BoxRadius`) true))