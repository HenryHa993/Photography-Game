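; Game state that runs Inkpot (Ink) dialogue stories and links them to the player's quest log.
; AssignStoryAsset creates the dialogue widget, begins the story and binds external functions that let Ink add quests and query their ongoing or completed status.
; The story-begin event passes the story to the widget for display.
; SwitchFlowToPath changes Ink flow, then jumps to a path and continues if the switch succeeds or Restart is set.
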(event `self.ReceiveBeginPlay`
  (bind _returnvalue (subsystem `Inkpot`))
  ;[1 1 1] Bind Inkpot Events OnBeginStory OnEndStory
  (add `Inkpot.EventOnStoryBegin` _returnvalue (delegate `Event OnStoryBegin`))
  (add `Inkpot.EventOnStoryEnd` _returnvalue (delegate `Event OnStoryEnd`)))

(event `Event OnStoryBegin`
  (params (Story :type "InkpotStory Object Reference"))
  ;[1 1 1] Bind Inkpot Events: OnStoryBegin, OnStoryEnd - UC: GameState, should be init on begin play
  (`DialogueWidget.ShowStory` (`self.Dialogue Display`) Story))

(event `Event OnStoryEnd`
  (params (Story :type "InkpotStory Object Reference"))
  ;[1 1 1] Bind Inkpot Events: OnStoryBegin, OnStoryEnd - UC: GameState, should be init on begin play
)

(fn `AssignQuest`
  (params (Values :type "Array of InkpotValue Structure (by ref)"))
  (returns (ReturnValue :type "InkpotValue Structure"))
  (bind _asbp_photo_character_base (cast `/Game/Core/Characters/Player/BP_PhotoCharacterBase` (`GameplayStatics.GetPlayerPawn` 0)))
  (bind _returnvalue (`QuestLogComponent.AddQuest` (`/Game/Core/Characters/Player/BP_PhotoCharacterBase.QuestLog` _asbp_photo_character_base) (`KismetStringLibrary.Conv_StringToName` (`InkpotLibrary.InkpotArrayValueAsString` Values))))
  (return (`InkpotLibrary.MakeBoolInkpotValue` _returnvalue)))

(fn `AssignStoryAsset`
  (params (`Story Asset` :type "InkpotStoryAsset Object Reference"))
  (set `self.Story Asset` `Story Asset`)
  ;[1 1 1] Create Dialogue Widget
  (bind _returnvalue (`|CreateWidget` "/Game/Core/DialogueSystem/WBP_Dialogue.WBP_Dialogue_C"))
  (bind _output_get (set `self.Dialogue Display` _returnvalue))
  (`UserWidget.AddToViewport` _output_get 0)
  (bind _returnvalue_2 (`Inkpot.BeginStory` (subsystem `Inkpot`) (`self.Story Asset`)))
  (bind _output_get_2 (set `self.Story` _returnvalue_2))
  ;[1 1 1] Setup External Functions
  (`InkpotStory.BindExternalFunction` _output_get_2 "AssignQuest" (`|CreateDelegate` :!event `AssignQuest`) true)
  (`InkpotStory.BindExternalFunction` _output_get_2 "CheckQuestAssigned" (`|CreateDelegate` :!event `Check Quest Assigned`) true)
  (`InkpotStory.BindExternalFunction` _output_get_2 "CheckQuestComplete" (`|CreateDelegate` :!event `CheckQuestComplete`) true))

(fn `Check Quest Assigned`
  (params (Values :type "Array of InkpotValue Structure (by ref)"))
  (returns (ReturnValue :type "InkpotValue Structure"))
  (bind _asbp_photo_character_base (cast `/Game/Core/Characters/Player/BP_PhotoCharacterBase` (`GameplayStatics.GetPlayerCharacter` 0)))
  (bind _returnvalue (`QuestLogComponent.CheckQuestOngoing` (`/Game/Core/Characters/Player/BP_PhotoCharacterBase.QuestLog` _asbp_photo_character_base) (`KismetStringLibrary.Conv_StringToName` (`InkpotLibrary.InkpotArrayValueAsString` Values))))
  (return (`InkpotLibrary.MakeBoolInkpotValue` _returnvalue)))

(fn `CheckQuestComplete`
  (params (Values :type "Array of InkpotValue Structure (by ref)"))
  (returns (ReturnValue :type "InkpotValue Structure"))
  (bind _asbp_photo_character_base (cast `/Game/Core/Characters/Player/BP_PhotoCharacterBase` (`GameplayStatics.GetPlayerPawn` 0)))
  (bind _returnvalue (`QuestLogComponent.CheckQuestComplete` (`/Game/Core/Characters/Player/BP_PhotoCharacterBase.QuestLog` _asbp_photo_character_base) (`KismetStringLibrary.Conv_StringToName` (`InkpotLibrary.InkpotArrayValueAsString` Values))))
  (return (`InkpotLibrary.MakeBoolInkpotValue` _returnvalue)))

(fn `SwitchFlowToPath`
  (params (Flow :type String) (Path :type String) (Restart :type Boolean))
  (bind _story (`self.Story`))
  (bind _returnvalue (`InkpotStory.SwitchFlow` (`self.Story`) Flow))
  (if _returnvalue
    (`InkpotStory.ChoosePath` _story Path :!label _label)
    (if (`InkpotStory.CanContinue` _story)
      (`InkpotStory.Continue` _story))
    (elif Restart
      (goto _label))))

(fn `UserConstructionScript`)