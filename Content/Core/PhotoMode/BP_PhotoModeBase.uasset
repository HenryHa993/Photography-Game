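; Base photo-mode pawn that swaps in its own UI and input for zooming and photographing clues, then re-possesses the player character on exit.
; Tick tests each BP_ClueBase for screen centering, a zoom-plus-distance score and line of sight, toggling its focus crosshair and tracking it as a subject.
; Capture renders a SceneCapture2D to a new render target, saves it with those subjects as a journal BP_PhotoEntry, and triggers flash and preview effects.
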(event `self.ReceiveBeginPlay`
  (bind _returnvalue (pcsubsystem `EnhancedInputLocalPlayerSubsystem` (`GameplayStatics.GetPlayerController` 0)))
  ;[1 1 1] Enter Photo Mode -> Add UI / Add IMC / Hide Other Widgets
  (bind _outactors (`GameplayStatics.GetAllActorsOfClass` "/Game/Core/PhotoMode/BP_ClueBase.BP_ClueBase_C"))
  (set `self.AllPhotoSubjects` _outactors)
  (bind _returnvalue_2 (`|CreateWidget` "/Game/Core/PhotoMode/UI/WBP_PhotoModeUIBase.WBP_PhotoModeUIBase_C"))
  (bind _output_get (set `self.PhotoUI` _returnvalue_2))
  (`UserWidget.AddToViewport` _output_get 0)
  (`/Engine/EditorBlueprintResources/StandardMacros.IsValid` _returnvalue
    (:`Is Valid`
      (`EnhancedInputSubsystemInterface.AddMappingContext` _returnvalue "/Game/Developers/Clayton/PhotoMode/PhotoModeControls/Input/IMC_PhotoModeControls.IMC_PhotoModeControls" 0 (struct))
      (`EnhancedInputSubsystemInterface.RemoveMappingContext` _returnvalue "/Game/Developers/Clayton/PhotoMode/Character/Input/IMC_Player3rdP.IMC_Player3rdP" (struct))
      (bind _foundwidgets (`WidgetBlueprintLibrary.GetAllWidgetsOfClass` "/Game/Developers/Clayton/PhotoMode/Clue/Interact/W_InteractionPrompt.W_InteractionPrompt_C" false))
      (`Widget.SetVisibility` _foundwidgets "Hidden"))))

(event `EnhancedInput|/Game/Developers/Clayton/PhotoMode/PhotoModeControls/Input/InputActions/IA_PM_ExitPhotoMode`
  (params (ActionValue :type Boolean) (ElapsedSeconds :type "Float (double-precision)") (TriggeredSeconds :type "Float (double-precision)") (InputAction :type "InputAction Object Reference" :default "/Game/Developers/Clayton/PhotoMode/PhotoModeControls/Input/InputActions/IA_PM_ExitPhotoMode.IA_PM_ExitPhotoMode"))
  (bind _returnvalue (`GameplayStatics.GetPlayerController` 0))
  (bind _returnvalue_2 (pcsubsystem `EnhancedInputLocalPlayerSubsystem` _returnvalue))
  ;[1 1 1] Back to Player Character
  (:`Started`
    (bind _returnvalue_3 (`GameplayStatics.GetActorOfClass` "/Game/Core/Characters/Player/BP_PhotoCharacterBase.BP_PhotoCharacterBase_C"))
    (`Controller.Possess` _returnvalue _returnvalue_3)
    (`EnhancedInputSubsystemInterface.RemoveMappingContext` _returnvalue_2 "/Game/Developers/Clayton/PhotoMode/PhotoModeControls/Input/IMC_PhotoModeControls.IMC_PhotoModeControls" (struct))
    (`EnhancedInputSubsystemInterface.AddMappingContext` _returnvalue_2 "/Game/Developers/Clayton/PhotoMode/Character/Input/IMC_Player3rdP.IMC_Player3rdP" 0 (struct))
    (`self.K2_DestroyActor`)
    (`Widget.RemoveFromParent` (stale `self.ReceiveBeginPlay` _output_get))
    (`self.SetActorHiddenInGame` _returnvalue_3 false)
    (set `/Game/Core/Characters/Player/BP_PhotoCharacterBase.IsCameraActive` false _returnvalue_3)
    (`Widget.SetVisibility` (stale `self.ReceiveBeginPlay` _foundwidgets) "Visible")
    (for _array_element (`self.AllPhotoSubjects`)
      (bind _asbp_clue_base (cast `/Game/Core/PhotoMode/BP_ClueBase` _array_element))
      (`/Game/Core/PhotoMode/UI/BP_FocusCrosshair.DeactivateCrosshair` (`/Game/Core/PhotoMode/BP_ClueBase.BP_FocusCrosshair` _asbp_clue_base)))))

(event `EnhancedInput|/Game/Developers/Clayton/PhotoMode/PhotoModeControls/Input/InputActions/IA_PM_Zoom_IN`
  (params (ActionValue :type Boolean) (ElapsedSeconds :type "Float (double-precision)") (TriggeredSeconds :type "Float (double-precision)") (InputAction :type "InputAction Object Reference" :default "/Game/Developers/Clayton/PhotoMode/PhotoModeControls/Input/InputActions/IA_PM_Zoom_IN.IA_PM_Zoom_IN"))
  ;[1 1 1] Zoom Function
  (:`Triggered`
    (bind _output_get (set `self.CurrentFOV` (`KismetMathLibrary.FClamp` (- (`self.CurrentFOV`) (`self.ZoomSpeed`)) 10.0 100.0)))
    (bind _output_get_2 (set `SceneCaptureComponent2D.FOVAngle` _output_get (`self.SceneCaptureComponent2D`)))
    (`CameraComponent.SetFieldOfView` (`self.Camera`) _output_get_2)))

(event `EnhancedInput|/Game/Developers/Clayton/PhotoMode/PhotoModeControls/Input/InputActions/IA_PM_Zoom_OUT`
  (params (ActionValue :type Boolean) (ElapsedSeconds :type "Float (double-precision)") (TriggeredSeconds :type "Float (double-precision)") (InputAction :type "InputAction Object Reference" :default "/Game/Developers/Clayton/PhotoMode/PhotoModeControls/Input/InputActions/IA_PM_Zoom_OUT.IA_PM_Zoom_OUT"))
  ;[1 1 1] Zoom Function
  (:`Triggered`
    (bind _output_get (set `self.CurrentFOV` (`KismetMathLibrary.FClamp` (+ (`self.CurrentFOV`) (`self.ZoomSpeed`)) 10.0 100.0)))
    (bind _output_get_2 (set `SceneCaptureComponent2D.FOVAngle` _output_get (`self.SceneCaptureComponent2D`)))
    (`CameraComponent.SetFieldOfView` (`self.Camera`) _output_get_2)))

(event `EnhancedInput|/Game/Developers/Clayton/PhotoMode/PhotoModeControls/Input/InputActions/IA_PM_CapturePhoto`
  (params (ActionValue :type Boolean) (ElapsedSeconds :type "Float (double-precision)") (TriggeredSeconds :type "Float (double-precision)") (InputAction :type "InputAction Object Reference" :default "/Game/Developers/Clayton/PhotoMode/PhotoModeControls/Input/InputActions/IA_PM_CapturePhoto.IA_PM_CapturePhoto"))
  ;[1 1 1] Capture Photo
  (:`Started`
    (`self.TakePhoto`)))

(event `self.ReceiveTick`
  (params (DeltaSeconds :type "Float (single-precision)"))
  ;[1 1 1] Crosshair tick
  (for _array_element (`self.AllPhotoSubjects`)
    (bind (_medal_score _score) (`self.GetScoreTarget` _array_element))
    (if (> _score 50)
      (bind _score_2 (`self.GetIndicatorScore` _array_element))
      (if (>= _score_2 12.0)
        (bind _outhit (`KismetSystemLibrary.LineTraceSingle` (`SceneComponent.K2_GetComponentLocation` (`self.Camera`)) (`SceneComponent.K2_GetComponentLocation` (`Actor.RootComponent` _array_element)) "TraceTypeQuery1"))
        (if (== (`.HitActor` (`GameplayStatics.BreakHitResult` _outhit)) _array_element)
          (`/Game/Core/PhotoMode/UI/BP_FocusCrosshair.ActivateCrosshair` (`/Game/Core/PhotoMode/BP_ClueBase.BP_FocusCrosshair` _array_element))
          (`KismetArrayLibrary.Array_AddUnique` (`self.PhotoSubjectRefArray`) _array_element)
          (else
            (`/Game/Core/PhotoMode/UI/BP_FocusCrosshair.DeactivateCrosshair` (`/Game/Core/PhotoMode/BP_ClueBase.BP_FocusCrosshair` _array_element) :!label _label)
            (`KismetArrayLibrary.Array_RemoveItem` (`self.PhotoSubjectRefArray`) _array_element)))
        (else
          (goto _label)))
      (else
        (goto _label)))))

(fn `CalculateMedalScore`
  (params (Score :type Integer))
  (returns (MedalScore :type String))
  (if (and (>= Score 1) (<= Score 50))
    (set `self.MedalScore` "BRONZE")
    (return (`self.MedalScore`))
    (elif (and (>= Score 51) (<= Score 85))
      (set `self.MedalScore` "SILVER")
      (return (`self.MedalScore`))
      (elif (and (>= Score 1) (<= Score 100))
        (set `self.MedalScore` "GOLD")
        (return (`self.MedalScore`))))))

(fn `CalculateScoreDistance`
  (params (ScreenLocation_X :type "Float (double-precision)") (ScreenLocation_Y :type "Float (double-precision)") (ScreenCenter_X :type "Float (double-precision)") (ScreenCenter_Y :type "Float (double-precision)"))
  (returns (ScoreDistance :type Integer))
  (bind _returnvalue (- ScreenLocation_Y ScreenCenter_Y))
  (bind _returnvalue_2 (- ScreenLocation_X ScreenCenter_X))
  ;[1 1 1] Distance From Centre = sqrt (  ( SLocation X - SCenter X ) ^2 + ( SLocation Y - SCenter Y ) ^2  )
  (bind _output_get (set `self.DistanceFromScreenCenter` (`KismetMathLibrary.Sqrt` (+ (* _returnvalue_2 _returnvalue_2) (* _returnvalue _returnvalue)))))
  (bind _output_get_2 (set `self.ScreenDiagonal` (`KismetMathLibrary.Sqrt` (+ (* ScreenCenter_X ScreenCenter_X) (* ScreenCenter_Y ScreenCenter_Y)))))
  ;[1 1 1] Normalized Distance = Distance / Screen Diagonal
  (bind _output_get_3 (set `self.NormalizedDistance` (/ _output_get _output_get_2)))
  (bind _output_get_4 (set `self.ScoreDistance` (`KismetMathLibrary.Round` (* (- 1.0 _output_get_3) 100.0))))
  (return _output_get_4))

(fn `GetFOV`
  (returns (UICurrentFOV :type "Float (double-precision)"))
  (return (`self.CurrentFOV`)))

(fn `GetIndicatorScore`
  (params (Actor :type "Actor Object Reference"))
  (returns (Score :type "Float (double-precision)"))
  (return (+ (/ 200.0 (`CameraComponent.FieldOfView` (`self.Camera`))) (/ 10000.0 (`KismetMathLibrary.Vector_Distance` (`SceneComponent.K2_GetComponentLocation` (`self.Camera`)) (`self.K2_GetActorLocation` Actor))))))

(fn `GetScoreTarget`
  (params (Target :type "Actor Object Reference"))
  (returns (`Medal Score` :type String) (Score :type Integer))
  (bind (_returnvalue_x _returnvalue_y) (`KismetMathLibrary.BreakVector2D` (`WidgetLayoutLibrary.GetViewportSize`)))
  (bind _screenlocation (`PlayerController.ProjectWorldLocationToScreen` (`GameplayStatics.GetPlayerController` 0) (`SceneComponent.K2_GetComponentLocation` (`Actor.RootComponent` Target)) false))
  (bind _scoredistance (`self.CalculateScoreDistance` (`KismetMathLibrary.BreakVector2D` _screenlocation) (`.Y` (`KismetMathLibrary.BreakVector2D` _screenlocation)) (/ _returnvalue_x 2.0) (/ _returnvalue_y 2.0)))
  (bind _medalscore (`self.CalculateMedalScore` _scoredistance))
  (return _medalscore _scoredistance))

(fn `SavePhoto`
  (bind _returnvalue (`KismetRenderingLibrary.CreateRenderTarget2D` 252 252))
  (set `TextureRenderTarget.TargetGamma` 1.3 _returnvalue)
  (set `SceneCaptureComponent2D.TextureTarget` _returnvalue (`self.SceneCaptureComponent2D`))
  (`SceneCaptureComponent2D.CaptureScene` (`self.SceneCaptureComponent2D`))
  ;[1 1 1] Parse in entry for photo instead of raw photo
  (bind _returnvalue_2 (`|SpawnActorFromClass` "/Game/Core/PhotoMode/Photo/BP_PhotoEntry.BP_PhotoEntry_C" (`KismetMathLibrary.MakeTransform` (0.0 0.0 0.0)) "Undefined" "MultiplyWithRoot" null (`SceneCaptureComponent2D.TextureTarget` (`self.SceneCaptureComponent2D`)) null))
  (set `/Game/Core/PhotoMode/Photo/BP_PhotoEntry.QuestItemsInPhoto` (`self.PhotoSubjectRefArray`) _returnvalue_2)
  (`KismetArrayLibrary.Array_AddUnique` (`/Game/Core/JournalSystem/W_Journal.PhotoEntries` (`/Game/Core/Characters/Player/BP_PhotoCharacterBase.JournalWidget` (`self.Player`))) _returnvalue_2))

(fn `TakePhoto`
  (`self.SavePhoto`)
  (bind _foundwidgets (`WidgetBlueprintLibrary.GetAllWidgetsOfClass` "/Game/Core/PhotoMode/UI/WBP_PhotoModeUIBase.WBP_PhotoModeUIBase_C" false))
  (`/Game/Core/PhotoMode/UI/WBP_PhotoModeUIBase.FlashEffectEvent` _foundwidgets)
  (bind _foundwidgets_2 (`WidgetBlueprintLibrary.GetAllWidgetsOfClass` "/Game/Developers/Clayton/PhotoMode/PhotoModeControls/WBP_Preview_Photo.WBP_Preview_Photo_C" false))
  (`/Game/Developers/Clayton/PhotoMode/PhotoModeControls/WBP_Preview_Photo.PreviewFadeEvent` _foundwidgets_2))

(fn `UserConstructionScript`)