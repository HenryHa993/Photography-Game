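; Base player character that handles photo mode, dialogue starts and the journal.
; E, while the journal is closed, starts an overlapped dialogue character's flow and removes third-person input, or otherwise spawns and possesses a photo-mode actor and hides the character.
; The journal widget is created collapsed at BeginPlay and toggled by input.
; Camera events re-attach FollowCamera to fixed virtual-camera actors; older spline-follow logic is disconnected.
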(event `NewPhotoMode`
  (params (ClueTransform :type "Transform Structure") (PhotoSubjectClassRef :type "Actor Class Reference"))
  ;[1 1 1] Spawns and Possesses Photo Mode
  (bind _returnvalue (`|SpawnActorFromClass` "/Game/Core/PhotoMode/BP_PhotoModeBase.BP_PhotoModeBase_C" (`self.GetTransform`) "Undefined" "MultiplyWithRoot" null self null))
  (`Controller.Possess` (`GameplayStatics.GetPlayerController` 0) _returnvalue)
  (`self.SetActorHiddenInGame` true)
  (set `self.IsCameraActive` true))

(event `Key|E`
  (params (Key :type "Key Structure"))
  (bind _overlappingactors (`self.GetOverlappingActors` "/Game/Developers/henry/Collections/JournalQuestIntegration/Blueprints/BP_DialogueCharacter.BP_DialogueCharacter_C"))
  ;[1 1 1] Open camera
  (:`Pressed`
    (if (`/Game/Core/JournalSystem/W_Journal.IsJournalOpen` (`self.JournalWidget`))
      _
      (elif (`KismetArrayLibrary.Array_IsNotEmpty` _overlappingactors)
        (bind _asbp_dialogue_character (cast `/Game/Developers/henry/Collections/JournalQuestIntegration/Blueprints/BP_DialogueCharacter` (`|GetArrayItem` _overlappingactors)))
        (bind _asbp_story_game_state_base (cast `/Game/Core/PhotoMode/BP_StoryGameStateBase` (`GameplayStatics.GetGameState`)))
        (`/Game/Core/PhotoMode/BP_StoryGameStateBase.SwitchFlowToPath` _asbp_story_game_state_base "Dialogue" (`/Game/Developers/henry/Collections/JournalQuestIntegration/Blueprints/BP_DialogueCharacter.CharacterName` _asbp_dialogue_character) true)
        (`EnhancedInputSubsystemInterface.RemoveMappingContext` (pcsubsystem `EnhancedInputLocalPlayerSubsystem` (`GameplayStatics.GetPlayerController` 0)) "/Game/Developers/Clayton/PhotoMode/Character/Input/IMC_Player3rdP.IMC_Player3rdP" (struct))
        (else
          (`self.NewPhotoMode` (struct)))))))

(event `self.ReceiveBeginPlay`
  ;[1 1 1] Set up journal
  (bind _returnvalue (`|CreateWidget` "/Game/Core/JournalSystem/W_Journal.W_Journal_C"))
  (bind _output_get (set `self.JournalWidget` _returnvalue))
  (`UserWidget.AddToViewport` _output_get 0)
  (`Widget.SetVisibility` _output_get "Collapsed"))

(event `EnhancedInput|/Game/Core/Input/Actions/IA_Journal`
  (params (ActionValue :type Boolean) (ElapsedSeconds :type "Float (double-precision)") (TriggeredSeconds :type "Float (double-precision)") (InputAction :type "InputAction Object Reference" :default "/Game/Core/Input/Actions/IA_Journal.IA_Journal"))
  (:`Triggered`
    (`/Game/Core/JournalSystem/W_Journal.Open/CloseJournal` (`self.JournalWidget`))))

(event `MoveCamera_01`
  (bind _returnvalue (`GameplayStatics.GetActorOfClass` "/Game/Developers/Clayton/CameraSystem/VirtualCameras/BP_VC_01.BP_VC_01_C"))
  (`SceneComponent.K2_AttachToComponent` (`self.FollowCamera`) (`/Game/Developers/Clayton/CameraSystem/VirtualCameras/BP_VC_01.FwdArrow` _returnvalue) "None" "KeepRelative" "KeepRelative" "KeepRelative" true))

(event `self.ReceiveTick`
  (params (DeltaSeconds :type "Float (single-precision)"))
  ;[1 1 1] *OLD* Move Camera to Spline
)

(event `MoveCamera_02`
  (bind _returnvalue (`GameplayStatics.GetActorOfClass` "/Game/Developers/Clayton/CameraSystem/VirtualCameras/BP_VC_02.BP_VC_02_C"))
  (`SceneComponent.K2_AttachToComponent` (`self.FollowCamera`) (`/Game/Developers/Clayton/CameraSystem/VirtualCameras/BP_VC_02.FwdArrow` _returnvalue) "None" "KeepRelative" "KeepRelative" "KeepRelative" true))

(fn `UserConstructionScript`)