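; BP_FairyCreature is a Fairy Forest level actor that animates a fairy around its starting pose with a vertical and yaw motion.
; On BeginPlay it caches its location and rotation, then plays a Timeline.
; Each update offsets Z and yaw from that pose by the same curve value scaled by RotationAmplitude, so height and turn move in lockstep.
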(event `self.ReceiveBeginPlay`
  (bind _output_get (set `self.FairyLocation` (`self.K2_GetActorLocation`)))
  (bind _output_get_2 (set `self.FairyRotation` (`self.K2_GetActorRotation`)))
  (bind (_direction _newtrack) (`Timeline|Timeline`)
    (:`Update`
      (`self.K2_SetActorTransform` (`KismetMathLibrary.MakeTransform` (`KismetMathLibrary.MakeVector` (.x _output_get) (.y _output_get) (+ (.z _output_get) (* _newtrack (`self.RotationAmplitude`)))) (`KismetMathLibrary.MakeRotator` (.roll _output_get_2) (.pitch _output_get_2) (+ (.yaw _output_get_2) (* (- _newtrack 0.0) (`self.RotationAmplitude`)))))))))

(fn `UserConstructionScript`)