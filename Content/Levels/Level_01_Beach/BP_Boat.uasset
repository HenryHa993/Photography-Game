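; BP_Boat is a boat actor in the Beach level that bobs and sways in place.
; On BeginPlay it caches its starting location and rotation, then plays a Timeline.
; Each update, one Timeline track drives both a height offset scaled by BobbingAmplitude and a pitch swing centered on the start rotation, scaled by SwayingAmplitude.
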(event `self.ReceiveBeginPlay`
  (bind _output_get (set `self.BoatLocation` (`self.K2_GetActorLocation`)))
  (bind _output_get_2 (set `self.BoatRotation` (`self.K2_GetActorRotation`)))
  (bind (_direction _newtrack_2) (`Timeline|Timeline`)
    (:`Update`
      (`self.K2_SetActorTransform` (`KismetMathLibrary.MakeTransform` (`KismetMathLibrary.MakeVector` (.x _output_get) (.y _output_get) (+ (.z _output_get) (* _newtrack_2 (`self.BobbingAmplitude`)))) (`KismetMathLibrary.MakeRotator` (.roll _output_get_2) (+ (.pitch _output_get_2) (* (- _newtrack_2 0.5) (`self.SwayingAmplitude`))) (.yaw _output_get_2)))))))

(fn `UserConstructionScript`)